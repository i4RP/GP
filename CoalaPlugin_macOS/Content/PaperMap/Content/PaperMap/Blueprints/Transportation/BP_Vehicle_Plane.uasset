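; BP_Vehicle_Plane is a plane vehicle that switches its animation between moving and stationary flight states.
; On BeginPlay it caches the AnimBP_Plane instance and places the collision component to match the starting FlightState.
; Each Tick compares the current location with the last one to detect movement, flips FlightState accordingly, and teleports the collision high up while moving or back to the origin when stopped.
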(event `self.ReceiveBeginPlay`
  (bind _collision (`self.Collision`))
  ;[1 1 1] Get Animation Blueprint
  (`parent.ReceiveBeginPlay`)
  (bind _asanim_bp_plane (cast `/ThoughtfishCoalaPlugin/PaperMap/Content/PaperMap/Animations/Transportation/AnimBP_Plane` (`SkeletalMeshComponent.GetAnimInstance` (`self.Plane`))))
  (bind _output_get (set `self.AnimBP` _asanim_bp_plane))
  (switch `int` (`/ThoughtfishCoalaPlugin/PaperMap/Content/PaperMap/Animations/Transportation/AnimBP_Plane.FlightState` _output_get)
    (:`Default`
      (`SceneComponent.K2_SetRelativeLocation` _collision (0.0 0.0 0.0) false true :!label _label))
    (:`0`
      (`SceneComponent.K2_SetRelativeLocation` _collision (0.0 0.0 11300.0) false true))
    (:`1`
      (goto _label))))

(event `self.ReceiveTick`
  (params (DeltaSeconds :type "Float (single-precision)"))
  (bind _animbp (`self.AnimBP`))
  (bind _collision (`self.Collision`))
  (bind _flightstate (`/ThoughtfishCoalaPlugin/PaperMap/Content/PaperMap/Animations/Transportation/AnimBP_Plane.FlightState` _animbp))
  ;[1 1 1] Update Plane Animation State
  (`|ExecutionSequence`
    (:`then_0`
      (`/Engine/EditorBlueprintResources/StandardMacros.IsValid` (`self.AnimBP`)
        (:`Is Valid`
          (if (`KismetMathLibrary.NearlyEqual_FloatFloat` (`KismetMathLibrary.Vector_Distance` (`self.LastPos`) (`self.K2_GetActorLocation`)))
            (if (== _flightstate 0)
              (set `/ThoughtfishCoalaPlugin/PaperMap/Content/PaperMap/Animations/Transportation/AnimBP_Plane.FlightState` 1 _animbp)
              (`SceneComponent.K2_SetRelativeLocation` _collision (0.0 0.0 0.0) false true))
            (elif (== _flightstate 1)
              (set `/ThoughtfishCoalaPlugin/PaperMap/Content/PaperMap/Animations/Transportation/AnimBP_Plane.FlightState` 0 _animbp)
              (`SceneComponent.K2_SetRelativeLocation` _collision (0.0 0.0 11300.0) false true))))))
    (:`then_1`
      (`parent.ReceiveTick` DeltaSeconds))
    (:`then_2`
      (set `self.LastPos` (`self.K2_GetActorLocation`)))))

(fn `UserConstructionScript`
  (`parent.UserConstructionScript`))
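; BP_Vehicle_Bus is a bus vehicle Blueprint that animates the bus according to whether it is moving.
; On BeginPlay it caches the AnimBP_Bus instance from the Bus mesh, calling the parent BeginPlay only if that cast succeeds.
; Each Tick compares the actor's location with the previous frame's to set IsDriving on the animation Blueprint, then runs the parent Tick.
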(event `self.ReceiveBeginPlay`
  ;[1 1 1] Get Animation Blueprint
  (bind _asanim_bp_bus (cast `/ThoughtfishCoalaPlugin/PaperMap/Content/PaperMap/Animations/Transportation/AnimBP_Bus` (`SkeletalMeshComponent.GetAnimInstance` (`self.Bus`))))
  (set `self.AnimBP` _asanim_bp_bus)
  (`parent.ReceiveBeginPlay`))

(event `self.ReceiveTick`
  (params (DeltaSeconds :type "Float (single-precision)"))
  ;[1 1 1] Update Animation
  (`|ExecutionSequence`
    (:`then_0`
      (`/Engine/EditorBlueprintResources/StandardMacros.IsValid` (`self.AnimBP`)
        (:`Is Valid`
          (set `/ThoughtfishCoalaPlugin/PaperMap/Content/PaperMap/Animations/Transportation/AnimBP_Bus.IsDriving` (not (== (`self.K2_GetActorLocation`) (`self.lastFramePos`))) (`self.AnimBP`)))))
    (:`then_1`
      (set `self.lastFramePos` (`self.K2_GetActorLocation`)))
    (:`then_2`
      (`parent.ReceiveTick` DeltaSeconds))))

(fn `UserConstructionScript`)
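; Train vehicle Blueprint that bends its carriage parts to follow the actor's turns as it moves.
; Tick samples rotation at an interval inversely scaled to the distance just travelled, keeping the last three samples.
; Two AnimBP_Train bone rotators lerp toward the newest and previous samples, so the second trails the first.
; BeginPlay and a stationary train snap both bones back to the actor's rotation with an axis offset.
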(event `ResetRotation`
  (bind _animbp (`self.AnimBP`))
  (bind _returnvalue (`KismetMathLibrary.MakeRotator` (+ (.roll (`self.K2_GetActorRotation`)) 90.0) (- (.pitch (`self.K2_GetActorRotation`)) 90.0) (.yaw (`self.K2_GetActorRotation`))))
  ;[1 1 1] Reset Train parts rotation
  (set `/ThoughtfishCoalaPlugin/PaperMap/Content/PaperMap/Animations/Transportation/AnimBP_Train.Bone1Rotator` _returnvalue _animbp)
  (set `/ThoughtfishCoalaPlugin/PaperMap/Content/PaperMap/Animations/Transportation/AnimBP_Train.Bone2Rotator` _returnvalue _animbp)
  (set `self.LerpEndRotBone1` _returnvalue)
  (set `self.LerpEndRotBone2` _returnvalue))

(event `self.ReceiveBeginPlay`
  ;[1 1 1] Init
  (set `self.LerpCounter` (`self.IntervallLength`))
  (bind _asanim_bp_train (cast `/ThoughtfishCoalaPlugin/PaperMap/Content/PaperMap/Animations/Transportation/AnimBP_Train` (`SkeletalMeshComponent.GetAnimInstance` (`self.Train`)))
    (:`then`
      (set `self.AnimBP` _asanim_bp_train))
    (:`CastFailed`
      _))
  (`parent.ReceiveBeginPlay`)
  (`KismetSystemLibrary.Delay` 0.005)
  (`self.ResetRotation`))

(event `self.ReceiveTick`
  (params (DeltaSeconds :type "Float (single-precision)"))
  (bind _animbp (`self.AnimBP`))
  (bind _lastthreerotations (`self.LastThreeRotations`))
  (bind _lastthreerotations_2 (`self.LastThreeRotations`))
  (bind _lastthreerotations_3 (`self.LastThreeRotations`))
  (bind _returnvalue (`KismetArrayLibrary.Array_Length` _lastthreerotations_2))
  (bind _returnvalue_2 (`KismetMathLibrary.Vector_Distance` (`self.LastPosition`) (`self.K2_GetActorLocation`)))
  ;[1 1 1] Animate Train Parts Rotation
  (`|ExecutionSequence`
    (:`then_0`
      (if (`self.UpdateSpeed`)
        (set `self.UpdateSpeed` false)
        (if (== _returnvalue_2 0.0)
          (set `self.CurrentSpeed` 0.5)
          (else
            (set `self.CurrentSpeed` (* (/ 1.0 _returnvalue_2) 0.1))))
        (set `self.IntervallLength` (`self.CurrentSpeed`))
        (if (>= (`KismetArrayLibrary.Array_Length` _lastthreerotations) 3)
          (`KismetArrayLibrary.Array_Remove` _lastthreerotations))
        (`KismetArrayLibrary.Array_Add` _lastthreerotations (`self.K2_GetActorRotation`))
        (set `self.LerpCounter` 0.0)
        (`|ExecutionSequence`
          (:`then_0`
            (bind _output_get (set `self.StartTurningBone1` (>= _returnvalue 2)))
            (if _output_get
              (set `self.LerpStartRotBone1` (`self.LerpEndRotBone1`))
              (set `self.LerpEndRotBone1` (`KismetMathLibrary.MakeRotator` (+ (.roll (`|GetArrayItem` _lastthreerotations_2 (- _returnvalue 1))) 90.0) (- (.pitch (`|GetArrayItem` _lastthreerotations_2 (- _returnvalue 1))) 90.0) (.yaw (`|GetArrayItem` _lastthreerotations_2 (- _returnvalue 1)))))))
          (:`then_1`
            (bind _output_get_2 (set `self.StartTurningBone2` (>= (`KismetArrayLibrary.Array_Length` (`self.LastThreeRotations`)) 3)))
            (if _output_get_2
              (set `self.LerpStartRotBone2` (`self.LerpEndRotBone2`))
              (set `self.LerpEndRotBone2` (`KismetMathLibrary.MakeRotator` (+ (.roll (`|GetArrayItem` _lastthreerotations_3 (- (`KismetArrayLibrary.Array_Length` _lastthreerotations_3) 2))) 90.0) (- (.pitch (`|GetArrayItem` _lastthreerotations_3 (- (`KismetArrayLibrary.Array_Length` _lastthreerotations_3) 2))) 90.0) (.yaw (`|GetArrayItem` _lastthreerotations_3 (- (`KismetArrayLibrary.Array_Length` _lastthreerotations_3) 2))))))))))
    (:`then_1`
      (`/Engine/EditorBlueprintResources/StandardMacros.IsValid` _animbp
        (:`Is Valid`
          (if (`self.StartTurningBone2`)
            (if (!= (`self.IntervallLength`) 0.5)
              (set `/ThoughtfishCoalaPlugin/PaperMap/Content/PaperMap/Animations/Transportation/AnimBP_Train.Bone2Rotator` (`KismetMathLibrary.RLerp` (`self.LerpStartRotBone2`) (`self.LerpEndRotBone2`) (`self.LerpCounter`) true) (`self.AnimBP`)))))))
    (:`then_2`
      (`/Engine/EditorBlueprintResources/StandardMacros.IsValid` _animbp
        (:`Is Valid`
          (if (`self.StartTurningBone1`)
            (if (!= (`self.IntervallLength`) 0.5)
              (set `/ThoughtfishCoalaPlugin/PaperMap/Content/PaperMap/Animations/Transportation/AnimBP_Train.Bone1Rotator` (`KismetMathLibrary.RLerp` (`self.LerpStartRotBone1`) (`self.LerpEndRotBone1`) (`self.LerpCounter`) true) (`self.AnimBP`))
              (set `self.LerpCounter` (+ (`self.LerpCounter`) (* (/ 1.0 (`self.IntervallLength`)) DeltaSeconds)))
              (else
                (`self.ResetRotation`)))))))
    (:`then_3`
      (bind _output_get_3 (set `self.Counter` (+ (`self.Counter`) DeltaSeconds)))
      (if (>= _output_get_3 (`self.IntervallLength`))
        (set `self.Counter` 0.0)
        (set `self.LastPosition` (`self.K2_GetActorLocation`))
        (set `self.UpdateSpeed` true)))
    (:`then_4`
      (`parent.ReceiveTick` DeltaSeconds))))

(fn `UserConstructionScript`)
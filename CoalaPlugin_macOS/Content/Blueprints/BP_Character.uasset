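; Player character for a Coala GPS map game, handling the map camera and point-of-interest selection.
; GPS changes become scene positions sent to player replication, while Coala scaling adjusts actor size, walk speed and boom length.
; POI clicks toggle info widgets and fly the boom between POI and player, reusing one timeline in both directions.
; Separate timelines handle manual zoom and top-down route view; Tick optionally follows a target between animations.
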(event `self.ReceiveBeginPlay`
  ;[0 0.03417 1] Begin Play
  ;[0 1 0.1122] Setup Player
  (`TimelineComponent.SetPlayRate` (`self.TL_ZoomtoActor`) 1.6)
  (`TimelineComponent.SetPlayRate` (`self.ZoomCamera`) 1.6)
  (bind (_notexist _coalabp) (`/ThoughtfishCoalaPlugin/Blueprints/Library/BP_BF_Coala.GetCoalaBP` self))
  (if (not _notexist)
    (`self.Try to Send Local Player Update` (`/ThoughtfishCoalaPlugin/Blueprints/BP_Coala.PlayerCurrentLon` _coalabp) (`/ThoughtfishCoalaPlugin/Blueprints/BP_Coala.PlayerCurrentLat` _coalabp))
    (add `/ThoughtfishCoalaPlugin/Blueprints/BP_Coala.GpsPositionChanged_0` _coalabp (delegate `OnGpsPositionChanged`))
    (`self.CoalaScaling`)
    (set `CharacterMovementComponent.MaxWalkSpeed` (`.Float` (`/ThoughtfishCoalaPlugin/Blueprints/Library/BP_BF_Coala.GetFloatByCoalaScaling` self (`CharacterMovementComponent.MaxWalkSpeed` (`self.CharacterMovement`)))) (`self.CharacterMovement`))
    (set `self.TempStartPointZoom` (`SceneComponent.K2_GetComponentLocation` (`self.CameraBoom`)))
    (set `self.TempArmLengthZoom` (`.Float` (`/ThoughtfishCoalaPlugin/Blueprints/Library/BP_BF_Coala.GetFloatByCoalaScaling` self (`self.ZoomedInCamera`))))
    (set `SpringArmComponent.TargetArmLength` (`.Float` (`/ThoughtfishCoalaPlugin/Blueprints/Library/BP_BF_Coala.GetFloatByCoalaScaling` self (`self.CameraArmLength`))) (`self.CameraBoom`))
    (set `self.ZoomedOutRotation` (`SceneComponent.K2_GetComponentRotation` (`self.CameraBoom`)))
    (set `self.TempCameraBoomRelativePos` (- (`self.K2_GetActorLocation`) (`SceneComponent.K2_GetComponentLocation` (`self.CameraBoom`))))
    (set `self.TempCameraBoomRotDefault` (`SceneComponent.K2_GetComponentRotation` (`self.CameraBoom`)))
    (set `self.TempTargetArmLengthDefault` (`SpringArmComponent.TargetArmLength` (`self.CameraBoom`)))))

(event `self.BPOnPoiInteract`
  (params (actor :type "CoalaInteractableActor Object Reference") (clickedOnInteractable :type Boolean))
  (bind _currentclickedpoi (`self.CurrentClickedPOI`))
  (bind _currentclickedpoi_2 (`self.CurrentClickedPOI`))
  (bind _currentclickedpoi_3 (`self.CurrentClickedPOI`))
  (bind _currentclickedpoi_4 (`self.CurrentClickedPOI`))
  ;[1 1 1] POIS Interact
  (cast `/ThoughtfishCoalaPlugin/Blueprints/Transportation/BP_Stop` (`self.CurrentClickedPOI`)
    (:`CastFailed`
      (bind _asbp_poi (cast `/ThoughtfishCoalaPlugin/Blueprints/BP_Poi` actor)
        (:`then`
          (if (`self.ZoomAnimationRunning`)
            _
            (elif (`self.CameraIsZoomedToPOI`)
              (if clickedOnInteractable :!label _label
                (`/Engine/EditorBlueprintResources/StandardMacros.IsValid` _currentclickedpoi_4
                  (:`Is Valid`
                    (if (!= _currentclickedpoi_4 _asbp_poi)
                      (if (`self.CameraIsZoomedToPOI`)
                        (`self.ZoomToLocation` (`SceneComponent.K2_GetComponentLocation` (`/ThoughtfishCoalaPlugin/Blueprints/BP_Poi.ZoomPoint` _asbp_poi)) (`/ThoughtfishCoalaPlugin/Blueprints/BP_Poi.ZoomRotate` _asbp_poi))
                        (`/ThoughtfishCoalaPlugin/Blueprints/BP_Poi.HideWidget` (`self.CurrentClickedPOI`) :!label _label_2)
                        (`self.EventFollowTarget` false)
                        (else
                          (`/Engine/EditorBlueprintResources/StandardMacros.IsValid` _currentclickedpoi_3 :!label _label_3
                            (:`Is Valid`
                              (if (!= _currentclickedpoi_3 _asbp_poi)
                                (goto _label_2)
                                (else
                                  _)))
                            (:`Is Not Valid`
                              _))))))
                  (:`Is Not Valid`
                    _))
                (`/ThoughtfishCoalaPlugin/Blueprints/BP_Poi.TogglePoiInfo` _asbp_poi)
                (bind _output_get (set `self.CurrentClickedPOI` _asbp_poi))
                (set `self.CurrentWidget` (`/ThoughtfishCoalaPlugin/Blueprints/BP_Poi.Widget` _output_get))
                (else
                  (`/Engine/EditorBlueprintResources/StandardMacros.IsValid` _currentclickedpoi_2
                    (:`Is Valid`
                      (bind _isvisible (`/ThoughtfishCoalaPlugin/Blueprints/BP_Poi.IsWidgetVisble` _currentclickedpoi_2))
                      (if _isvisible
                        (`self.ZoomToPlayer` :!label _label_4)
                        (else
                          (if (`self.CameraIsZoomedToPOI`) :!label _label_5
                            (goto _label_4)
                            (else
                              (if (`self.IsShowingRoute`) :!label _label_6
                                (cast `/ThoughtfishCoalaPlugin/Blueprints/Transportation/BP_Stop` _currentclickedpoi_2
                                  (:`then`
                                    _)
                                  (:`CastFailed`
                                    (goto _label_4)))))))))
                    (:`Is Not Valid`
                      (goto _label_6)))
                  (`/Engine/EditorBlueprintResources/StandardMacros.IsValid` _currentclickedpoi :!label _label_7
                    (:`Is Valid`
                      (`/ThoughtfishCoalaPlugin/Blueprints/BP_Poi.HideWidget` _currentclickedpoi)))))
              (elif clickedOnInteractable
                (goto _label_3)
                (else
                  (goto _label_7))))))
        (:`CastFailed`
          (if (not (`self.ZoomAnimationRunning`))
            (goto _label)))))))

(event `DisableMovement`
  ;[1 1 1] Set Movement
  (`CharacterMovementComponent.DisableMovement` (`self.CharacterMovement`)))

(event `OnGpsPositionChanged`
  (params (zoom :type Byte) (long :type "Float (double-precision)") (lat :type "Float (double-precision)"))
  ;[0 1 0.1122] Setup Player
  (`self.Try to Send Local Player Update` long lat))

(event `SetMovement`
  (params (NewMovementMode :type "EMovementMode Enum" :default "MOVE_None"))
  ;[1 1 1] Set Movement
  (`CharacterMovementComponent.SetMovementMode` (`self.CharacterMovement`) NewMovementMode 0))

(event `CoalaScaling`
  (bind _cameraboom (`self.CameraBoom`))
  ;[1 0 0] Coala Scaling
  (`self.SetActorScale3D` (`.Vector` (`/ThoughtfishCoalaPlugin/Blueprints/Library/BP_BF_Coala.GetVectorByCoalaScaling` self (1.0 1.0 1.0))))
  (`/Engine/EditorBlueprintResources/StandardMacros.IsValid` _cameraboom
    (:`Is Valid`
      (set `SpringArmComponent.TargetArmLength` (`.Float` (`/ThoughtfishCoalaPlugin/Blueprints/Library/BP_BF_Coala.GetFloatByCoalaScaling` self (`self.CameraArmLength`))) _cameraboom))))

(event `Event Close Current Widget`
  ;[1 1 1] POIS Interact
  (`|ExecutionSequence`
    (:`then_0`
      (goto _label_5))
    (:`then_1`
      (set `self.CurrentClickedPOI` null)
      (set `self.CurrentWidget` null))))

(event `ObjectWasCleanedUp`
  (bind _currentclickedpoi (`self.CurrentClickedPOI`))
  ;[1 1 1] POIS Interact
  (cast `/ThoughtfishCoalaPlugin/Blueprints/Transportation/BP_Vehicle` _currentclickedpoi)
  (`/Engine/EditorBlueprintResources/StandardMacros.IsValid` _currentclickedpoi
    (:`Is Valid`
      (`/ThoughtfishCoalaPlugin/Blueprints/BP_Poi.HideWidget` _currentclickedpoi))
    (:`Is Not Valid`
      (`/ThoughtfishCoalaPlugin/Blueprints/WI_POI_Coala.HideWidget` (`self.CurrentWidget`))))
  (if (or (`self.CameraIsZoomedToPOI`) (`self.IsShowingRoute`))
    (`self.ZoomToPlayer`)))

(event `InputAction|ZoomIn`
  (params (Key :type "Key Structure"))
  (bind _cameraboom (`self.CameraBoom`))
  ;[0.2921 0.3274 1] zoom in/out
  (:`Pressed`
    (if (not (`self.BlockZoom`))
      (set `self.ZoomAnimationRunning` true)
      (if (`self.CameraIsZoomed`)
        (set `self.CameraIsZoomed` false)
        (bind (_direction _zoom) (`Timeline|ZoomCamera` :!via `Reverse` :!label _label_8)
          (:`Update`
            (`/Engine/EditorBlueprintResources/StandardMacros.IsValid` _cameraboom
              (:`Is Valid`
                (set `SpringArmComponent.TargetArmLength` (`KismetMathLibrary.Lerp` (`.Float` (`/ThoughtfishCoalaPlugin/Blueprints/Library/BP_BF_Coala.GetFloatByCoalaScaling` self (`self.ZoomedInCamera`))) (`.Float` (`/ThoughtfishCoalaPlugin/Blueprints/Library/BP_BF_Coala.GetFloatByCoalaScaling` self (`self.CameraArmLength`))) _zoom) _cameraboom)
                (`SceneComponent.K2_SetWorldRotation` _cameraboom (`KismetMathLibrary.MakeRotator` 0.0 (`KismetMathLibrary.Lerp` (.pitch (`self.ZoomedInRotation`)) (.pitch (`self.ZoomedOutRotation`)) _zoom)) false false))))
          (:`Finished`
            (set `self.ZoomAnimationRunning` false)))
        (else
          (set `self.CameraIsZoomed` true)
          (goto _label_8))))))

(event `ZoomOut`
  (bind _cameraboom (`self.CameraBoom`))
  ;[0.2921 0.3274 1] zoom in/out
  (`/ThoughtfishCoalaPlugin/Blueprints/WI_POI_Coala.HideWidget` (`self.CurrentWidget`))
  (set `self.CameraIsZoomedToPOI` false)
  (set `self.BlockZoom` true)
  (set `self.IsShowingRoute` true)
  (set `self.ZoomAnimationRunning` true)
  (`self.EventFollowTarget` false)
  (bind (_direction _zoom) (`Timeline|Timeline_0` :!via `PlayFromStart`)
    (:`Update`
      (`/Engine/EditorBlueprintResources/StandardMacros.IsValid` _cameraboom
        (:`Is Valid`
          (set `SpringArmComponent.TargetArmLength` (`KismetMathLibrary.Lerp` (`.Float` (`/ThoughtfishCoalaPlugin/Blueprints/Library/BP_BF_Coala.GetFloatByCoalaScaling` self (`self.ZoomedOutCamera`))) (`.Float` (`/ThoughtfishCoalaPlugin/Blueprints/Library/BP_BF_Coala.GetFloatByCoalaScaling` self (`self.CameraArmLength`))) _zoom) _cameraboom)
          (`SceneComponent.K2_SetWorldRotation` _cameraboom (`KismetMathLibrary.MakeRotator` 0.0 (`KismetMathLibrary.Lerp` (.pitch (struct :`Pitch` -90.0)) (.pitch (`self.ZoomedOutRotation`)) _zoom)) false false))))
    (:`Finished`
      (set `self.BlockZoom` false)
      (set `self.ZoomAnimationRunning` false))))

(event `ZoomToLocation`
  (params (TempEndPointZoom :type "Vector Structure") (TempEndRotateZoom :type "Rotator Structure"))
  (bind _returnvalue (`SceneComponent.K2_GetComponentLocation` (`self.CameraBoom`)))
  (bind _returnvalue_2 (`SceneComponent.K2_GetComponentRotation` (`self.CameraBoom`)))
  ;[1 1 1] Zoom to Actor and Zoom to Player
  (if (not (`self.ZoomAnimationRunning`))
    (set `self.TempEndPointZoom` TempEndPointZoom)
    (set `self.TempEndRotateZoom` TempEndRotateZoom)
    (set `self.CameraIsZoomedToPOI` true)
    (set `self.ZoomAnimationRunning` true)
    (set `self.BlockZoom` true)
    (`self.DisableMovement`)
    (if (`self.IsShowingRoute`)
      (set `self.TempStartPointZoom` (`self.TempEndPointZoom`))
      (set `self.TempEndPointZoom` _returnvalue)
      (set `self.TempStartRotateZoom` _returnvalue_2)
      (set `self.TempArmLengthZoom` (`.Float` (`/ThoughtfishCoalaPlugin/Blueprints/Library/BP_BF_Coala.GetFloatByCoalaScaling` self (`self.ZoomedInCamera`))))
      (bind (_direction _move _zoom) (`Timeline|TL_ZoomtoActor` :!via `ReverseFromEnd` :!label _label_9)
        (:`Update`
          (`SceneComponent.K2_SetWorldLocation` (`self.CameraBoom`) (`KismetMathLibrary.VLerp` (`self.TempStartPointZoom`) (`self.TempEndPointZoom`) _move) false false)
          (if (`self.IsShowingRoute`)
            (set `SpringArmComponent.TargetArmLength` (`KismetMathLibrary.Lerp` (`.Float` (`/ThoughtfishCoalaPlugin/Blueprints/Library/BP_BF_Coala.GetFloatByCoalaScaling` self (`self.ZoomedOutCamera`))) (`self.TempArmLengthZoom`) _zoom) (`self.CameraBoom`))
            (else
              (set `SpringArmComponent.TargetArmLength` (`KismetMathLibrary.Lerp` (`.Float` (`/ThoughtfishCoalaPlugin/Blueprints/Library/BP_BF_Coala.GetFloatByCoalaScaling` self (`self.ZoomedInCamera`))) (`self.TempArmLengthZoom`) _zoom) (`self.CameraBoom`))))
          (`SceneComponent.K2_SetWorldRotation` (`self.CameraBoom`) (`KismetMathLibrary.RLerp` (`self.TempStartRotateZoom`) (`self.TempEndRotateZoom`) _move) false false))
        (:`Finished`
          (set `self.IsShowingRoute` false)
          (set `self.ZoomAnimationRunning` false)
          (if (not (`self.CameraIsZoomedToPOI`))
            (`self.SetMovement` "MOVE_Walking")
            (set `self.BlockZoom` false)
            (bind _output_get (set `self.TempStartPointZoom` (+ (`self.K2_GetActorLocation`) (`self.TempCameraBoomRelativePos`))))
            (`SceneComponent.K2_SetWorldLocation` (`self.CameraBoom`) _output_get false false))))
      (else
        (set `self.TempStartPointZoom` _returnvalue)
        (set `self.TempStartRotateZoom` _returnvalue_2)
        (set `self.TempArmLengthZoom` (`SpringArmComponent.TargetArmLength` (`self.CameraBoom`)))
        (goto _label_9 :!via `PlayFromStart`)))))

(event `ZoomToPlayer`
  ;[1 1 1] Zoom to Actor and Zoom to Player
  (if (not (`self.ZoomAnimationRunning`))
    (set `self.TempStartPointZoom` (+ (`self.K2_GetActorLocation`) (`self.TempCameraBoomRelativePos`)))
    (set `self.TempStartRotateZoom` (`self.TempCameraBoomRotDefault`))
    (set `self.TempArmLengthZoom` (`self.TempTargetArmLengthDefault`))
    (`self.EventFollowTarget` false)
    (set `self.TempEndPointZoom` (`SceneComponent.K2_GetComponentLocation` (`self.CameraBoom`)))
    (set `self.TempEndRotateZoom` (`SceneComponent.K2_GetComponentRotation` (`self.CameraBoom`)))
    ;;[1 1 1] Set Camera Zoom
    (set `self.CameraIsZoomed` false)
    (set `self.ZoomAnimationRunning` true)
    (set `self.BlockZoom` true)
    (set `self.CameraIsZoomedToPOI` false)
    (goto _label_9 :!via `ReverseFromEnd`)))

(event `self.ReceiveTick`
  (params (DeltaSeconds :type "Float (single-precision)"))
  ;[1 1 1] While zooming out the Camera will be updated with each player movement. (optional)
  (if (and (`self.FollowTarget`) (== (`self.ZoomAnimationRunning`) false))
    (`SceneComponent.K2_SetWorldLocation` (`self.CameraBoom`) (`SceneComponent.K2_GetComponentLocation` (`/ThoughtfishCoalaPlugin/Blueprints/BP_Poi.ZoomPoint` (`self.Target`))) false false)))

(event `EventFollowTarget`
  (params (FollowTarget :type Boolean) (Target :type "/ThoughtfishCoalaPlugin/Blueprints/BP_Poi Object Reference"))
  (bind _output_get (set `self.FollowTarget` FollowTarget))
  (if _output_get
    (set `self.Target` Target)))

(fn `Try to Send Local Player Update`
  (params (newPosLongitude :type "Float (double-precision)") (newPosLatitude :type "Float (double-precision)"))
  (bind _returnvalue (subsystem `CoalaPlayerReplication`))
  (`CoalaPlayerReplication.SetLocalPlayerCurrentLevelPosition` _returnvalue (`CoalaGpsConverterFunctionLibrary.ToScenePosition` newPosLongitude newPosLatitude))
  (`CoalaPlayerReplication.ScheduleRemotePlayerRefresh` _returnvalue false))

(fn `UserConstructionScript`
  (`self.CoalaScaling`))
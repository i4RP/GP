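; Example handler actor that sets up COALA player replication for showing remote players on the map.
; Once the COALA map loads, it sets a placeholder device-based local player ID, applies display range, refresh times, visibility and player class from its config, then enables the system.
; Player updates move default remote player actors to their new positions, while add and removal events are empty hooks for customization.
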(event `self.ReceiveBeginPlay`
  ;[1 1 1] Start as soon as the COALA map is ready
  (bind (_notexist _coalabp) (`/ThoughtfishCoalaPlugin/Blueprints/Library/BP_BF_Coala.GetCoalaBP` self))
  (if (not _notexist)
    (add `/ThoughtfishCoalaPlugin/Blueprints/BP_Coala.MapLoaded` _coalabp (delegate `OnMapLoaded`))))

(event `OnMapLoaded`
  (bind _returnvalue (subsystem `CoalaPlayerReplication`))
  ;[1 1 1] Provide a user id based on login or similar here, GetDeviceId does not work on all platforms
  (bind _localplayerid (`self.GetLocalPlayerId`))
  (`CoalaPlayerReplication.SetLocalPlayerId` _returnvalue _localplayerid)
  (`self.SetConfiguration`)
  ;[1 1 1] Add your customization here
  (`|ExecutionSequence`
    (:`then_0`
      (add `CoalaPlayerReplication.onNewPlayerAdded` _returnvalue (delegate `OnNewPlayerAdded`)))
    (:`then_1`
      (add `CoalaPlayerReplication.onPlayerBeginRemoval` _returnvalue (delegate `OnPlayerRemoved`)))
    (:`then_2`
      (add `CoalaPlayerReplication.onUpdatePlayer` _returnvalue (delegate `OnUpdatePlayer`))
      (`CoalaPlayerReplication.SetSystemEnabled` _returnvalue true))))

(event `OnUpdatePlayer`
  (params (playerData :type "CoalaRemotePlayerData Structure (by ref)") (player :type "Actor Object Reference") (newWorldPosition :type "Vector Structure (by ref)"))
  ;[1 1 1] Add your customization here
  (bind _asbp_coala_default_remote_player (cast `/ThoughtfishCoalaPlugin/Blueprints/PlayerReplication/BP_Coala_DefaultRemotePlayer` player))
  (`/ThoughtfishCoalaPlugin/Blueprints/PlayerReplication/BP_Coala_DefaultRemotePlayer.MoveToPosition` _asbp_coala_default_remote_player newWorldPosition))

(event `OnNewPlayerAdded`
  (params (playerData :type "CoalaRemotePlayerData Structure (by ref)") (player :type "Actor Object Reference"))
  ;[1 1 1] Add your customization here
)

(event `OnPlayerRemoved`
  (params (playerData :type "CoalaRemotePlayerData Structure (by ref)") (player :type "Actor Object Reference"))
  ;[1 1 1] Add your customization here
)

(fn `GetLocalPlayerId`
  (returns (LocalPlayerId :type String))
  (`KismetSystemLibrary.PrintString` "Implement your local player id generation!" true true (struct :`R` 1.0 :`G` 0.008024 :`A` 1.0) 3.0)
  (return (`CoalaPlatformMisc.GetDeviceIdForCurrentPlatform`)))

(fn `SetConfiguration`
  (bind _returnvalue (subsystem `CoalaPlayerReplication`))
  (bind _config_asset (`self.Config Asset`))
  (bind _config_asset_2 (`self.Config Asset`))
  (bind _config_asset_3 (`self.Config Asset`))
  (`CoalaPlayerReplication.SetDisplayRangeOfRemotePlayers` _returnvalue (`CoalaPlayerReplicationConfig.xRequestDistanceFromPlayerInMeters` _config_asset) (`CoalaPlayerReplicationConfig.yRequestDistanceFromPlayerInMeters` _config_asset) true)
  (`CoalaPlayerReplication.SetPlayerRefreshTimes` _returnvalue (`CoalaPlayerReplicationConfig.minimumSecondsBetweenPlayerRefreshes` _config_asset_3) (`CoalaPlayerReplicationConfig.maximumSecondsBetweenPlayerRefreshes` _config_asset_3))
  (`CoalaPlayerReplication.SetPlayerRefreshTimesWhenAlone` _returnvalue (`CoalaPlayerReplicationConfig.minimumSecondsBetweenPlayerRefreshesWhenAlone` _config_asset_2) (`CoalaPlayerReplicationConfig.maximumSecondsBetweenPlayerRefreshesWhenAlone` _config_asset_2))
  (`CoalaPlayerReplication.SetLocalPlayerVisibility` _returnvalue (`CoalaPlayerReplicationConfig.defaultLocalPlayerVisibility` (`self.Config Asset`)))
  (set `CoalaPlayerReplication.playerActorClass` (`self.PlayerClassToSpawn`) _returnvalue))

(fn `UserConstructionScript`)
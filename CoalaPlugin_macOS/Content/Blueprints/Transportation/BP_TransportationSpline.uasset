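; Transportation route actor that builds spline meshes along its spline for a bus, train or flight route.
; The UpdateSpline event runs only once, adding one spline mesh component per segment from a branch chosen by transport type.
; All branches share the same attach and shaping logic, matching each segment's points and tangents and scaling its cross-section by the Coala scale times 100.
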(event `UpdateSpline`
  (params (Type :type "TransportationType Enum" :default "NONE"))
  (bind _spline (`self.Spline`))
  (bind _splinemeshcomponent (`self.SplineMeshComponent`))
  (bind _splinescale (`self.SplineScale`))
  ;[1 1 1] Update Spline
  (`/Engine/EditorBlueprintResources/StandardMacros.DoOnce` false
    (:`Completed`
      (bind _returnvalue (`CoalaController.GetCoalaScale`))
      (bind _returnvalue_2 (* _returnvalue 100.0))
      (set `self.SplineScale` (`KismetMathLibrary.MakeVector2D` _returnvalue_2 _returnvalue_2))
      (for _index (range (+ (- (`SplineComponent.GetNumberOfSplinePoints` (`self.Spline`)) 2) 1))
        (switch `TransportationType` Type
          (:`BUS`
            (bind _returnvalue_3 (`AddComponent|NODE_AddSplineMeshComponent-1` :`bManualAttachment` true))
            (set `self.SplineMeshComponent` _returnvalue_3))
          (:`TRAIN`
            (bind _returnvalue_4 (`AddComponent|NODE_AddSplineMeshComponent-2` :`bManualAttachment` true))
            (set `self.SplineMeshComponent` _returnvalue_4))
          (:`FLIGHT`
            (bind _returnvalue_5 (`AddComponent|NODE_AddSplineMeshComponent-3` :`bManualAttachment` true))
            (set `self.SplineMeshComponent` _returnvalue_5)))
        (`SceneComponent.K2_AttachToComponent` (`self.SplineMeshComponent`) (`self.DefaultSceneRoot`) "None" "KeepRelative" "KeepRelative" "KeepRelative" true)
        (bind (_location _tangent) (`SplineComponent.GetLocationAndTangentAtSplinePoint` _spline _index "Local"))
        (bind (_location_2 _tangent_2) (`SplineComponent.GetLocationAndTangentAtSplinePoint` _spline (+ _index 1) "Local"))
        (`SplineMeshComponent.SetStartAndEnd` _splinemeshcomponent _location _tangent _location_2 _tangent_2 true)
        (`SplineMeshComponent.SetStartScale` _splinemeshcomponent _splinescale true)
        (`SplineMeshComponent.SetEndScale` _splinemeshcomponent _splinescale true)))))

(fn `UserConstructionScript`)
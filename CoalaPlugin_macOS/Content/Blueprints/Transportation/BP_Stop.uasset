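; Transit stop actor that shows a popup widget with stop and arrival info from the CoalaBP transportation data.
; Init takes a transport Type, resolves its StopId by looking itself up in that type's object set, then fills the widget with full stop info.
; ShowWidget refreshes arrivals only, then again when its timeline finishes; a comment intends 10-second updates, but no replay is wired.
; Inherited zoom-to-actor and zoom-to-player events are overridden empty to disable them.
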(event `Init`
  (params (Type :type "TransportationType Enum" :default "NONE"))
  (bind _widget (`self.Widget`))
  ;[1 1 1] Initiate Widget
  (set `self.type` Type)
  (bind (_notexist _coalabp) (`/ThoughtfishCoalaPlugin/Blueprints/Library/BP_BF_Coala.GetCoalaBP` self))
  (if _notexist
    (`KismetSystemLibrary.PrintString` "CoalaBPIsMissing")
    (else
      (bind _output_get (set `self.CoalaBP` _coalabp))
      (bind (_foundid _returnvalue) (`CoalaTransportation.FindStopIdFromObject` (`BlueprintMapLibrary.Map_Find` (`/ThoughtfishCoalaPlugin/Blueprints/BP_Coala.TransportationObjectSets` _output_get) (`self.type`)) self))
      (if _foundid
        (bind _output_get_2 (set `self.stopId` _returnvalue))
        (if (`self.UseWidget`)
          (`/Engine/EditorBlueprintResources/StandardMacros.IsValid` _widget
            (:`Is Valid`
              (bind _returnvalue_2 (`CoalaTransportation.GetStopPopupInfo` (`BlueprintMapLibrary.Map_Find` (`/ThoughtfishCoalaPlugin/Blueprints/BP_Coala.TransportationDataSets` (`self.CoalaBP`)) (`self.type`)) _output_get_2))
              (`/ThoughtfishCoalaPlugin/Blueprints/WI_POI_Coala.Event SetUpWidgetStop` _widget _returnvalue_2 false (`self.type`)))))))))

(event `self.ShowWidget`
  (bind _widget (`self.Widget`))
  (bind _widget_2 (`self.Widget`))
  (bind _value (`BlueprintMapLibrary.Map_Find` (`/ThoughtfishCoalaPlugin/Blueprints/BP_Coala.TransportationDataSets` (`self.CoalaBP`)) (`self.type`)))
  ;[1 1 1] Show Widget. Update Stop Popup Info every 10 seconds
  (if (`self.UseWidget`)
    (`/Engine/EditorBlueprintResources/StandardMacros.IsValid` _widget
      (:`Is Valid`
        (bind _returnvalue (`CoalaTransportation.GetStopPopupInfo` _value (stale `Init` _output_get_2) true))
        (`/ThoughtfishCoalaPlugin/Blueprints/WI_POI_Coala.Event SetUpWidgetStop` _widget _returnvalue true (`self.type`))
        (`parent.ShowWidget`)
        (`Timeline|Timeline_0` :!via `PlayFromStart`
          (:`Finished`
            (`/Engine/EditorBlueprintResources/StandardMacros.IsValid` _widget_2
              (:`Is Valid`
                (bind _returnvalue_2 (`CoalaTransportation.GetStopPopupInfo` _value (`self.stopId`) true))
                (`/ThoughtfishCoalaPlugin/Blueprints/WI_POI_Coala.Event SetUpWidgetStop` _widget_2 _returnvalue_2 true (`self.type`))))))))))

(event `self.ZoomToActor`
  ;[1 1 1] Disable those ParentEvents
)

(event `self.ReceiveTick`
  (params (DeltaSeconds :type "Float (single-precision)"))
  (`parent.ReceiveTick` DeltaSeconds))

(event `self.ZoomToPlayer`
  ;[1 1 1] Disable those ParentEvents
)

(fn `UserConstructionScript`
  (`parent.UserConstructionScript`))
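; Player controller that turns touch input into GPS-based movement targets for the player through the Coala Blueprint.
; Pressing or moving the first finger reads the GPS hit location under the cursor, writes it as target latitude and longitude, and sets the movement-pressed flag.
; Releasing any finger clears that flag, and both paths first check that the Coala Blueprint exists.
; A separate actor touch event only prints a debug string.
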(event `self.ReceiveBeginPlay`
  (`/ThoughtfishCoalaPlugin/Blueprints/Library/BP_BF_Coala.GetCoalaBP` self))

(event `self.ReceiveActorOnInputTouchBegin`
  (params (FingerIndex :type "ETouchIndex Enum" :default "Touch1"))
  (`KismetSystemLibrary.PrintString` "Hello"))

(event `InputTouch`
  (params (Location :type "Vector Structure") (FingerIndex :type "ETouchIndex Enum"))
  (:`Pressed`
    (switch `ETouchIndex` FingerIndex :!label _label
      (:`Touch1`
        (bind _returnvalue (`self.GetGpsHitLocationUnderCursor`))
        (bind (_notexist _coalabp) (`/ThoughtfishCoalaPlugin/Blueprints/Library/BP_BF_Coala.GetCoalaBP` self))
        (if (not _notexist)
          (set `/ThoughtfishCoalaPlugin/Blueprints/BP_Coala.buttonForMovementPressed` true _coalabp)
          (bind (_lon _lat) (`CoalaGPSCoordinatesBlueprintLibrary.BreakCoalaGPSCoordinates` _returnvalue))
          (set `/ThoughtfishCoalaPlugin/Blueprints/BP_Coala.PlayerTargetLat` _lat _coalabp)
          (set `/ThoughtfishCoalaPlugin/Blueprints/BP_Coala.PlayerTargetLon` _lon _coalabp)))))
  (:`Released`
    (bind (_notexist_2 _coalabp_2) (`/ThoughtfishCoalaPlugin/Blueprints/Library/BP_BF_Coala.GetCoalaBP` self))
    (if (not _notexist_2)
      (set `/ThoughtfishCoalaPlugin/Blueprints/BP_Coala.buttonForMovementPressed` false _coalabp_2)))
  (:`Moved`
    (goto _label)))

(fn `UserConstructionScript`)
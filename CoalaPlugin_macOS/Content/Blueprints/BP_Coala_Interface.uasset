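; Interface actor for the COALA map plugin that creates the loading, player and optional GPS movement widgets.
; On BeginPlay it can show loading and lock player input, then binds to BP_Coala and player events.
; Area events update loading text; map completion restores input and removes the loading screen.
; Position, weather and time updates target WI_Player_Coala through UIWidget, whose assignment here is disconnected from execution.
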(event `self.ReceiveBeginPlay`
  (bind _movementwidget (`self.MovementWidget`))
  (bind _player (`self.Player`))
  (bind _player_2 (`self.Player`))
  (bind (_player_3 _exist) (`/ThoughtfishCoalaPlugin/Blueprints/Library/BP_BF_Coala.GetCoalaPlayer` self))
  (if _exist
    (set `self.Player` _player_3))
  (if (`self.ShowLoading`)
    (`/Engine/EditorBlueprintResources/StandardMacros.IsValid` _player
      (:`Is Valid`
        (`self.DisableInput` _player (`GameplayStatics.GetPlayerController` 0)))
      (:`Is Not Valid`
        _))
    (bind _returnvalue (`|CreateWidget` (`self.LoadingWidget`)))
    (bind _output_get (set `self.UILoading` _returnvalue))
    (`UserWidget.AddToViewport` _output_get 10))
  (bind _returnvalue_2 (`|CreateWidget` (`self.PlayerWidget`)))
  (`UserWidget.AddToViewport` _returnvalue_2 0)
  (bind (_notexist _coalabp) (`/ThoughtfishCoalaPlugin/Blueprints/Library/BP_BF_Coala.GetCoalaBP` self))
  (set `self.refToCoalaBP` _coalabp)
  (if (not _notexist)
    (add `/ThoughtfishCoalaPlugin/Blueprints/BP_Coala.MapLoaded` (`self.refToCoalaBP`) (delegate `MapLoaded`))
    (add `/ThoughtfishCoalaPlugin/Blueprints/BP_Coala.RequestCoalaArea` (`self.refToCoalaBP`) (delegate `OnRequestCoalaArea`))
    (add `/ThoughtfishCoalaPlugin/Blueprints/BP_Coala.AreaLoaded` (`self.refToCoalaBP`) (delegate `OnAreaLoaded`)))
  (`/Engine/EditorBlueprintResources/StandardMacros.IsValid` _player_2
    (:`Is Valid`
      (add `/ThoughtfishCoalaPlugin/Blueprints/BP_Character.NewPlayerPostion` _player_2 (delegate `NewPlayerPostion`))
      (add `/ThoughtfishCoalaPlugin/Blueprints/BP_Coala.WeatherDataReceived` (`self.refToCoalaBP`) (delegate `WeatherUpdate`))
      ;[1 1 1] add GPS moving UI if available
      (if (`KismetSystemLibrary.IsValidClass` _movementwidget)
        (bind _returnvalue_3 (`|CreateWidget` _movementwidget))
        (`UserWidget.AddToViewport` _returnvalue_3 0)))))

(event `NewPlayerPostion`
  (params (Lon :type "Float (double-precision)") (Lat :type "Float (double-precision)"))
  ;[1 1 1] Update Coordinates
  (bind _aswi_player_coala (cast `/ThoughtfishCoalaPlugin/Blueprints/WI_Player_Coala` (`self.UIWidget`)))
  (`/ThoughtfishCoalaPlugin/Blueprints/WI_Player_Coala.UpdateLocation` _aswi_player_coala Lon Lat))

(event `OnRequestCoalaArea`
  (params (indexArea :type "CoalaTile Structure"))
  (if (`KismetSystemLibrary.IsValid` (`self.UILoading`))
    (`/ThoughtfishCoalaPlugin/Blueprints/WI_Loading_Coala.ChangeLoadingText` (`self.UILoading`) (`KismetStringLibrary.Concat_StrStr` "Request " (`KismetStringLibrary.Conv_IntToString` (`/ThoughtfishCoalaPlugin/Blueprints/BP_Coala.countAreasToCreateTillMapLoaded` (`self.refToCoalaBP`))) " COALA area data and generate map ..."))
    (else
      (remove `/ThoughtfishCoalaPlugin/Blueprints/BP_Coala.RequestCoalaArea` (`self.refToCoalaBP`) (delegate `OnRequestCoalaArea`)))))

(event `WeatherUpdate`
  (params (NewParam :type "/ThoughtfishCoalaPlugin/Blueprints/types/WeatherType Enum" :default "NewEnumerator0"))
  ;[1 1 1] When BP_coala received weather updates they are handled here.
  (bind _aswi_player_coala (cast `/ThoughtfishCoalaPlugin/Blueprints/WI_Player_Coala` (`self.UIWidget`)))
  (`/ThoughtfishCoalaPlugin/Blueprints/WI_Player_Coala.UpdateWeather` _aswi_player_coala NewParam))

(event `OnAreaLoaded`
  (params (Area :type "CoalaArea Object Reference"))
  (bind (_indexx _indexy) (`CoalaTileBlueprintLibrary.BreakCoalaTile` (`.coalaTile` (`CoalaAreaShadowingFix.BreakCoalaArea` Area))))
  (if (`KismetSystemLibrary.IsValid` (`self.UILoading`))
    (bind (_notexist _coalabp) (`/ThoughtfishCoalaPlugin/Blueprints/Library/BP_BF_Coala.GetCoalaBP` self))
    (if (not _notexist)
      (`/ThoughtfishCoalaPlugin/Blueprints/WI_Loading_Coala.ChangeLoadingText` (`self.UILoading`) (`KismetStringLibrary.Concat_StrStr` "Area " (`KismetStringLibrary.Conv_IntToString` _indexx) "_" (`KismetStringLibrary.Conv_IntToString` _indexy) " loaded " "( " (`KismetStringLibrary.Conv_IntToString` (`/ThoughtfishCoalaPlugin/Blueprints/BP_Coala.countAreasToCreateTillMapLoaded` _coalabp)) " more to do )")))))

(event `MapLoaded`
  (bind _player (`self.Player`))
  ;[1 1 1] If Map Loaded
  (bind _aswi_player_coala (cast `/ThoughtfishCoalaPlugin/Blueprints/WI_Player_Coala` (`self.UIWidget`))
    (:`then`
      (`/ThoughtfishCoalaPlugin/Blueprints/WI_Player_Coala.UpdateTime` _aswi_player_coala)
      (`/ThoughtfishCoalaPlugin/Blueprints/WI_Player_Coala.UpdateWeather` _aswi_player_coala "NewEnumerator0"))
    (:`CastFailed`
      _))
  (`/Engine/EditorBlueprintResources/StandardMacros.IsValid` _player
    (:`Is Valid`
      (`self.EnableInput` _player (`GameplayStatics.GetPlayerController` 0)))
    (:`Is Not Valid`
      _))
  ;;[0.9782 1 0.231] Remove Loading
  (`/Engine/EditorBlueprintResources/StandardMacros.IsValid` (`self.UILoading`)
    (:`Is Valid`
      (`Widget.RemoveFromParent` (`self.UILoading`)))))

(fn `UserConstructionScript`)
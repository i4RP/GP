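; BP_HeatMapToken is a single marker on the crime heat map, registered with its area and showing an accumulated weight.
; Init creates a dynamic material driven by a Weight parameter and offsets the mesh by a scale-corrected displaced center.
; Visibility requires weight above the configured threshold and a position inside loaded areas.
; For pillar heat maps, tick grows the Z scale to a weight-based height after a random delay, then disables itself.
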(event `self.ReceiveBeginPlay`)

(event `self.ReceiveTick`
  (params (DeltaSeconds :type "Float (single-precision)"))
  (if (`self.ShouldGrow`)
    (`self.SetActorScale3D` (`KismetMathLibrary.MakeVector` (.x (`self.GetActorScale3D`)) (.y (`self.GetActorScale3D`)) (`KismetMathLibrary.Lerp` (* 0.2 (`self.CoalaScale`)) (`self.ZScale`) (`self.LerpS`))))
    (if (>= (`self.LerpS`) 1.0)
      (set `self.ShouldGrow` false)
      (`self.SetActorTickEnabled` false)
      (else
        (set `self.LerpS` (`KismetMathLibrary.FClamp` (+ (* DeltaSeconds 0.5) (`self.LerpS`))))))))

(event `UpdateAfterInitComplete`
  (bind ((`heatMapType` _heatmaptype) (`pillarScale` _pillarscale)) (break `CoalaCrimeRenderConfig` (`self.CrimeRenderConfig`)))
  (`self.SetVisible` true)
  (switch `UHeatMapType` _heatmaptype
    (:`Pillar`
      (`KismetSystemLibrary.Delay` (`KismetMathLibrary.RandomFloatInRange` 0.0 2.0))
      (set `self.ZScale` (* (+ (* (`self.Weight`) _pillarscale) 1.0) (`self.CoalaScale`)))
      (set `self.LerpS` 0.0)
      (set `self.ShouldGrow` true)
      (`self.SetActorTickEnabled` true))))

(fn `AddWeight`
  (params (WeightToAdd :type "Float (double-precision)"))
  (bind _output_get (set `self.Weight` (+ (`self.Weight`) WeightToAdd)))
  (`MaterialInstanceDynamic.SetScalarParameterValue` (`self.DynamicMaterialInstance`) "Weight" _output_get)
  (`self.SetVisible` true))

(fn `Init`
  (params (Area :type "CoalaArea Object Reference") (DisplacedCenter :type "Vector Structure") (CrimeRenderConfig :type "CoalaCrimeRenderConfig Structure") (CoalaScale :type "Float (double-precision)"))
  (bind _staticmesh (`self.StaticMesh`))
  (bind _weight (`self.Weight`))
  (bind _staticmesh_2 (`self.StaticMesh`))
  (set `self.CoalaScale` CoalaScale)
  (`CoalaMeshGenerator.AddAttachedActorToHeatMap` Area self)
  (`self.SaveArea` Area)
  (bind _output_get (set `self.CrimeRenderConfig` CrimeRenderConfig))
  (bind _returnvalue (`KismetMaterialLibrary.CreateDynamicMaterialInstance` (`PrimitiveComponent.GetMaterial` _staticmesh 0)))
  (bind _output_get_2 (set `self.DynamicMaterialInstance` _returnvalue))
  (`PrimitiveComponent.SetMaterial` _staticmesh 0 _output_get_2)
  (`MaterialInstanceDynamic.SetScalarParameterValue` _output_get_2 "Weight" _weight)
  (if (<= _weight (`.weightThreshold` (break `CoalaCrimeRenderConfig` _output_get)))
    (`self.SetVisible` false))
  (`SceneComponent.K2_SetRelativeLocation` _staticmesh_2 (+ (* DisplacedCenter (/ 1.0 (`local.CoalaScale`))) (`SceneComponent.RelativeLocation` _staticmesh_2)) false true))

(fn `SaveArea`
  (params (`Coala Area` :type "CoalaArea Object Reference"))
  (set `self.Area` `Coala Area`))

(fn `SetVisible`
  (params (visible :type Boolean))
  (if (<= (`self.Weight`) (`.weightThreshold` (break `CoalaCrimeRenderConfig` (`self.CrimeRenderConfig`))))
    (`SceneComponent.SetVisibility` (`self.DefaultSceneRoot`) false true :!label _label)
    (elif (`self.IsOutsideLoadedAreas`)
      (goto _label)
      (else
        (`SceneComponent.SetVisibility` (`self.DefaultSceneRoot`) visible true)))))

(fn `UserConstructionScript`)
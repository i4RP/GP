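; Point-of-interest actor for the Coala player, scaled by the Coala scale, that shows an info widget with name, description and icon.
; Toggling shows or hides the widget, optionally zooming to the POI or back to the player and pausing movement.
; In Dynamic style, Tick projects a world anchor to screen space to position the widget.
; Sphere overlap with the Coala player sets the interactable flag.
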(event `self.ReceiveBeginPlay`
  ;[1 1 1] Set Coala Player
  (bind (_player _exist) (`/ThoughtfishCoalaPlugin/Blueprints/Library/BP_BF_Coala.GetCoalaPlayer` self))
  (if _exist
    (set `self.CoalaPlayer` _player))
  (if (`self.UseWidget`)
    (bind _returnvalue (`|CreateWidget` (`self.WidgetClass`)))
    (bind _aswi_poi_coala (cast `/ThoughtfishCoalaPlugin/Blueprints/WI_POI_Coala` _returnvalue))
    (bind _output_get (set `self.Widget` _aswi_poi_coala))
    (`/ThoughtfishCoalaPlugin/Blueprints/WI_POI_Coala.SetupWidget` _output_get (`self.PoiName`) (`self.PoiDescription`) (`self.PoiIcon`) (`self.WidgetSize`))))

(event `TogglePoiInfo`
  (if (`self.UseWidget`)
    (`/Engine/EditorBlueprintResources/StandardMacros.IsValid` (`self.Widget`)
      (:`Is Valid`
        (bind _isvisible (`self.IsWidgetVisble`))
        (if _isvisible
          (`self.HideWidget`)
          (`self.ZoomToPlayer`)
          (if (`self.StopMovementByShow`)
            (`/ThoughtfishCoalaPlugin/Blueprints/BP_Character.SetMovement` (`self.CoalaPlayer`) "MOVE_Walking"))
          (else
            (`self.ShowWidget`)
            (`self.ZoomToActor`)
            (if (`self.StopMovementByShow`)
              (`/ThoughtfishCoalaPlugin/Blueprints/BP_Character.DisableMovement` (`self.CoalaPlayer`)))))))))

(event `ShowWidget`
  (if (`self.UseWidget`)
    (`/Engine/EditorBlueprintResources/StandardMacros.IsValid` (`self.Widget`)
      (:`Is Valid`
        (`/ThoughtfishCoalaPlugin/Blueprints/WI_POI_Coala.ShowWidget` (`self.Widget`))))))

(event `HideWidget`
  (if (`self.UseWidget`)
    (`/Engine/EditorBlueprintResources/StandardMacros.IsValid` (`self.Widget`)
      (:`Is Valid`
        (`/ThoughtfishCoalaPlugin/Blueprints/WI_POI_Coala.HideWidget` (`self.Widget`))))))

(event `self.ReceiveTick`
  (params (DeltaSeconds :type "Float (single-precision)"))
  (bind (_screenposition _returnvalue) (`WidgetLayoutLibrary.ProjectWorldLocationToWidgetPosition` (`GameplayStatics.GetPlayerController` 0) (`SceneComponent.K2_GetComponentLocation` (`self.ShowWidgetPoint`))))
  (if (`self.UseWidget`)
    (`/Engine/EditorBlueprintResources/StandardMacros.IsValid` (`self.Widget`)
      (:`Is Valid`
        (switch `/ThoughtfishCoalaPlugin/Blueprints/types/POIWidgetStyle` (`self.WidgetStyle`)
          (:`NewEnumerator1`
            ;[1 1 1] Dynamic Widget
            (if (`Widget.IsInViewport` (`self.Widget`))
              (if _returnvalue
                (`UserWidget.SetPositionInViewport` (`self.Widget`) (+ _screenposition (`self.WidgetOffset`)) false)))))))))

(event `self.Sphere.OnComponentEndOverlap`
  (params (OverlappedComponent :type "PrimitiveComponent Object Reference") (OtherActor :type "Actor Object Reference") (OtherComp :type "PrimitiveComponent Object Reference") (OtherBodyIndex :type Integer))
  (bind _coalaplayer (`self.CoalaPlayer`))
  ;[1 1 1] Overlay Events
  (`/Engine/EditorBlueprintResources/StandardMacros.IsValid` _coalaplayer
    (:`Is Valid`
      (if (== _coalaplayer OtherActor)
        (set `self.IsInteractable` false)))))

(event `self.Sphere.OnComponentBeginOverlap`
  (params (OverlappedComponent :type "PrimitiveComponent Object Reference") (OtherActor :type "Actor Object Reference") (OtherComp :type "PrimitiveComponent Object Reference") (OtherBodyIndex :type Integer) (bFromSweep :type Boolean) (SweepResult :type "HitResult Structure (by ref)"))
  (bind _coalaplayer (`self.CoalaPlayer`))
  ;[1 1 1] Overlay Events
  (`/Engine/EditorBlueprintResources/StandardMacros.IsValid` _coalaplayer
    (:`Is Valid`
      (if (== _coalaplayer OtherActor)
        (set `self.IsInteractable` true)))))

(fn `CoalaScaling`
  (bind _returnvalue (`CoalaController.GetCoalaScale`))
  (`self.SetActorScale3D` (`KismetMathLibrary.MakeVector` _returnvalue _returnvalue _returnvalue)))

(fn `IsWidgetVisble`
  (returns (IsVisible :type Boolean))
  (`/Engine/EditorBlueprintResources/StandardMacros.IsValid` (`self.Widget`)
    (:`Is Valid`
      (return (`Widget.IsVisible` (`self.Widget`))))))

(fn `UserConstructionScript`
  (`self.CoalaScaling`))

(fn `ZoomToActor`
  (if (`self.ZoomToPOI`)
    (`/Engine/EditorBlueprintResources/StandardMacros.IsValid` (`self.CoalaPlayer`)
      (:`Is Valid`
        (`/ThoughtfishCoalaPlugin/Blueprints/BP_Character.ZoomToLocation` (`self.CoalaPlayer`) (`SceneComponent.K2_GetComponentLocation` (`self.ZoomPoint`)) (`self.ZoomRotate`)))
      (:`Is Not Valid`
        _)))
  (return))

(fn `ZoomToPlayer`
  (if (`self.ZoomToPOI`)
    (`/Engine/EditorBlueprintResources/StandardMacros.IsValid` (`self.CoalaPlayer`)
      (:`Is Valid`
        (`/ThoughtfishCoalaPlugin/Blueprints/BP_Character.ZoomToPlayer` (`self.CoalaPlayer`)))
      (:`Is Not Valid`
        _)))
  (return))
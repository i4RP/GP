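; Coala weather and sky controller that drives time-of-day lighting and switchable weather effects.
; Hours and minutes, taken from the system clock outside dev mode or a fast 24-hour preview event, drive the sky sphere, sun/moon directional light, moon opacity and MPC fog through curves.
; Weather changes fade out, swap and fade in player-attached particles via timelines; dev mode sets moon phase and binds to Coala weather data.
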(event `CallDayNightCycle`
  ;[0 0.04334 1] Call Day/ NIght Cycle
  (if (not (`self.DayNightCycleIsRunning`))
    (set `self.DayNightCycleIsRunning` true)
    (`/Engine/EditorBlueprintResources/StandardMacros.IsValid` (`self.SunDirectionalLight`)
      (:`Is Valid`
        (`/Engine/EditorBlueprintResources/StandardMacros.IsValid` (`self.SkySphere`)
          (:`Is Valid`
            (set `self.Hours` 0)
            (set `self.Minutes` 0)
            (if (< (`self.Hours`) 24) :!label _label
              (`self.UpdateManually`)
              (`KismetSystemLibrary.Delay` 0.0125)
              (`/Engine/EditorBlueprintResources/StandardMacros.IncrementInt` (`self.Minutes`)
                (:`  `
                  (if (> (`self.Minutes`) 59)
                    (`/Engine/EditorBlueprintResources/StandardMacros.IncrementInt` (`self.Hours`)
                      (:`  `
                        (set `self.Minutes` 0)
                        (goto _label)))
                    (else
                      (goto _label)))))
              (else
                (set `self.DayNightCycleIsRunning` false)))))))))

(event `ToChangeWeatherCalled`
  (params (NewParam :type "/ThoughtfishCoalaPlugin/Blueprints/types/WeatherType Enum" :default "NewEnumerator0"))
  ;[1 0.2174 0.3473] To Change Weather
  (if (not (`self.WeatherIsChanging`))
    (set `self.WeatherIsChanging` true)
    (`/Engine/EditorBlueprintResources/StandardMacros.IsValid` (`self.CurrentWeather`)
      (:`Is Valid`
        (bind (_direction _alpha) (`Timeline|TL_EndWeather` :!via `PlayFromStart`)
          (:`Update`
            (`ParticleSystemComponent.SetFloatParameter` (`self.CurrentWeather`) "PP_Weather_alpha" _alpha))
          (:`Finished`
            (`ActorComponent.K2_DestroyComponent` (`self.CurrentWeather`))
            (`self.ChangeWeather` NewParam :!label _label_2)
            (`/Engine/EditorBlueprintResources/StandardMacros.IsValid` (`self.CurrentWeather`)
              (:`Is Valid`
                (bind (_direction_2 _alpha_2) (`Timeline|TL_StartWeather` :!via `PlayFromStart`)
                  (:`Update`
                    (`ParticleSystemComponent.SetFloatParameter` (`self.CurrentWeather`) "PP_Weather_alpha" _alpha_2))
                  (:`Finished`
                    (set `self.WeatherIsChanging` false :!label _label_3))))
              (:`Is Not Valid`
                (goto _label_3))))))
      (:`Is Not Valid`
        (goto _label_2)))))

(event `UpdateManually`
  ;[1 1 1] Update Sun Manually
  (`self.SetupSkySphere`)
  (`self.SetDirectionLightPostion` (`self.Hours`) (`self.Minutes`))
  (`self.SetSunMoonIntensity` (`self.SunDirectionalLight`) (`self.CoalaSunIntensity`) (`self.CoalaSunColor`) (`self.Hours`) (`self.Minutes`))
  (`self.SetMoonOpacity` (`self.Hours`) (`self.Minutes`))
  (`self.SetFogColor` (`self.Hours`) (`self.Minutes`))
  (`self.SetFog`))

(event `StartRain`
  ;[1 1 1] Start Weather / Events
  (`self.ToChangeWeatherCalled` "NewEnumerator0"))

(event `self.ReceiveTick`
  (params (DeltaSeconds :type "Float (single-precision)"))
  (bind (_year _month _day _hour _minute) (`KismetMathLibrary.BreakDateTime` (`KismetMathLibrary.Now`)))
  (if (and (not (`self.UseDevmode`)) (not (`self.DayNightCycleIsRunning`)))
    (set `self.Hours` _hour)
    (set `self.Minutes` _minute)
    (`self.UpdateManually`)))

(event `StartSnow`
  ;[1 1 1] Start Weather / Events
  (`self.ToChangeWeatherCalled` "NewEnumerator7"))

(event `self.ReceiveBeginPlay`
  (`self.SetupLight`)
  (set `self.DayNightCycleIsRunning` false)
  (set `self.WeatherIsChanging` false)
  ;[1 1 1] Attach to player
  (bind (_player _exist) (`/ThoughtfishCoalaPlugin/Blueprints/Library/BP_BF_Coala.GetCoalaPlayer` self))
  (if _exist
    (`self.K2_AttachToActor` (`self.SkySphere`) _player "None" "SnapToTarget" "KeepRelative" "KeepRelative" true))
  (`KismetSystemLibrary.Delay` 0.2)
  (`self.UpdateManually`)
  (if (`self.UseDevmode`)
    (`self.SetMoonPhase` (`self.DevMoonPhase`))
    (bind (_notexist _coalabp) (`/ThoughtfishCoalaPlugin/Blueprints/Library/BP_BF_Coala.GetCoalaBP` self))
    (if (not _notexist)
      (add `/ThoughtfishCoalaPlugin/Blueprints/BP_Coala.WeatherDataReceived` _coalabp (delegate `ToChangeWeatherCalled`)))))

(event `StartMist`
  ;[1 1 1] Start Weather / Events
  (`self.ToChangeWeatherCalled` "NewEnumerator8"))

(event `StartClearSky`
  ;[1 1 1] Start Weather / Events
  (`self.ToChangeWeatherCalled` "NewEnumerator1"))

(event `SetMoonPhase`
  (params (MoonPhase :type "/ThoughtfishCoalaPlugin/Blueprints/types/MoonPhase Enum" :default "NewEnumerator5"))
  ;[1 1 1] Set Moon Phase
  (`self.SetMoonPhaseFn` MoonPhase))

(fn `ChangeWeather`
  (params (Selection :type "/ThoughtfishCoalaPlugin/Blueprints/types/WeatherType Enum" :default "NewEnumerator0"))
  (switch `/ThoughtfishCoalaPlugin/Blueprints/types/WeatherType` Selection
    (:`NewEnumerator0`
      ;[1 1 1] Rain
      (`self.SpawnWeatherParticalSystem` (`self.RainSetting`) :!label _label))
    (:`NewEnumerator1`
      (set `self.CurrentWeather` null :!label _label_2))
    (:`NewEnumerator2`
      (goto _label_2))
    (:`NewEnumerator3`
      (goto _label_2))
    (:`NewEnumerator4`
      (goto _label_2))
    (:`NewEnumerator5`
      (goto _label))
    (:`NewEnumerator6`
      (goto _label))
    (:`NewEnumerator7`
      ;[1 1 1] Snow
      (`self.SpawnWeatherParticalSystem` (`self.SnowSetting`)))
    (:`NewEnumerator8`
      ;[1 1 1] Mist
      (`self.SpawnWeatherParticalSystem` (`self.MistSetting`)))))

(fn `CoalaScaling`
  (`self.UpdateManually`))

(fn `GetMoonPostion`
  (params (Hours :type Integer) (Minutes :type Integer))
  (returns (InMoonPhase :type Boolean) (MoonRotation :type "Rotator Structure"))
  (bind _skysphere (`self.SkySphere`))
  (bind _arise (`self.IsMoonShowing` Hours Minutes))
  (if _arise
    (`/Engine/EditorBlueprintResources/StandardMacros.IsValid` _skysphere
      (:`Is Valid`
        (return true (`/ThoughtfishCoalaPlugin/Blueprints/BP_Sky_Sphere_Coala.MoonRotation` _skysphere)))
      (:`Is Not Valid`
        _)))
  (return false))

(fn `IsMoonArise `
  (params (Hours :type Integer))
  (returns (Arise :type Boolean))
  (if (`self.UseMoonMesh`)
    (return (or (== Hours (`self.MoonHoursTo`)) (== Hours (`self.MoonHoursFrom`))))
    (else
      (return false))))

(fn `IsMoonShowing`
  (params (Hours :type Integer) (Minutes :type Integer))
  (returns (Arise :type Boolean))
  (if (`self.UseMoonMesh`)
    (if (or (`KismetMathLibrary.InRange_IntInt` Hours 0 (`self.MoonHoursTo`)) (`KismetMathLibrary.InRange_IntInt` Hours (`self.MoonHoursFrom`) 24))
      (if (or (== Hours (`self.MoonHoursTo`)) (== Hours (`self.MoonHoursFrom`)))
        (if (== Hours (`self.MoonHoursTo`))
          (if (`KismetMathLibrary.InRange_IntInt` Minutes 0 (`self.MoonMinutesTo`))
            (return true)
            (else
              (return false)))
          (elif (`KismetMathLibrary.InRange_IntInt` Minutes (`self.MoonMinutesFrom`) 60)
            (return true)
            (else
              (return false))))
        (else
          (return true)))
      (else
        (return false)))
    (else
      (return false))))

(fn `SetDirectionLightPostion`
  (params (Hours :type Integer) (Minutes :type Integer))
  (bind (_inmoonphase _moonrotation) (`self.GetMoonPostion` Hours Minutes))
  (bind _skysphere (`self.SkySphere`))
  (bind _returnvalue (`KismetMathLibrary.Lerp` 0.0 15.0 (/ (`KismetMathLibrary.Conv_IntToDouble` Minutes) 60.0)))
  (bind _returnvalue_2 (`KismetMathLibrary.Lerp` 0.0 360.0 (/ (`KismetMathLibrary.Conv_IntToDouble` Hours) 24.0)))
  (`/Engine/EditorBlueprintResources/StandardMacros.IsValid` (`self.SunDirectionalLight`)
    (:`Is Valid`
      (`/Engine/EditorBlueprintResources/StandardMacros.IsValid` _skysphere
        (:`Is Valid`
          (set `/ThoughtfishCoalaPlugin/Blueprints/BP_Sky_Sphere_Coala.SunCurvePos` (`KismetMathLibrary.MapRangeUnclamped` (+ _returnvalue_2 _returnvalue) 0.0 360.0 0.0 24.0) _skysphere)
          (if _inmoonphase
            (set `/ThoughtfishCoalaPlugin/Blueprints/BP_Sky_Sphere_Coala.IgnorMoonUpdate` false (`self.SkySphere`))
            (set `/ThoughtfishCoalaPlugin/Blueprints/BP_Sky_Sphere_Coala.IgnorSunUpdate` true (`self.SkySphere`))
            ;[0 0.3498 1] Set Moon Light
            (`self.K2_SetActorRotation` (`self.SunDirectionalLight`) _moonrotation false)
            (set `/ThoughtfishCoalaPlugin/Blueprints/BP_Sky_Sphere_Coala.SunHeightNightOffset` -1.0 (`self.SkySphere`))
            (else
              (bind _arise (`self.IsMoonArise ` Hours))
              (if _arise
                (set `/ThoughtfishCoalaPlugin/Blueprints/BP_Sky_Sphere_Coala.IgnorMoonUpdate` false (`self.SkySphere`))
                (else
                  (set `/ThoughtfishCoalaPlugin/Blueprints/BP_Sky_Sphere_Coala.IgnorMoonUpdate` true (`self.SkySphere`))))
              (set `/ThoughtfishCoalaPlugin/Blueprints/BP_Sky_Sphere_Coala.IgnorSunUpdate` false (`self.SkySphere`))
              ;[0 0.3498 1] Set Sun Light
              (`self.K2_SetActorRotation` (`self.SunDirectionalLight`) (`KismetMathLibrary.MakeRotator` 0.0 (+ _returnvalue_2 _returnvalue 90.0)) false)
              (set `/ThoughtfishCoalaPlugin/Blueprints/BP_Sky_Sphere_Coala.SunHeightNightOffset` 0.0 (`self.SkySphere`))))
          (`/Engine/EngineSky/BP_Sky_Sphere.UpdateSunDirection` (`self.SkySphere`)))))))

(fn `SetFog`
  (set `PostProcessComponent.bEnabled` (`self.UseFog`) (`self.PP_Fog`))
  (`KismetMaterialLibrary.SetScalarParameterValue` "/ThoughtfishCoalaPlugin/Materials/MPC.MPC" "FogDenstityDistance" (`.Float` (`/ThoughtfishCoalaPlugin/Blueprints/Library/BP_BF_Coala.GetFloatByCoalaScaling` self (`self.FogDensityDistance`))))
  (`KismetMaterialLibrary.SetScalarParameterValue` "/ThoughtfishCoalaPlugin/Materials/MPC.MPC" "FogStartDistance" (`.Float` (`/ThoughtfishCoalaPlugin/Blueprints/Library/BP_BF_Coala.GetFloatByCoalaScaling` self (`self.Fog Start Distance`))))
  (`KismetMaterialLibrary.SetScalarParameterValue` "/ThoughtfishCoalaPlugin/Materials/MPC.MPC" "Fog Height" (`.Float` (`/ThoughtfishCoalaPlugin/Blueprints/Library/BP_BF_Coala.GetFloatByCoalaScaling` self (`self.Fog Height`))))
  (`KismetMaterialLibrary.SetScalarParameterValue` "/ThoughtfishCoalaPlugin/Materials/MPC.MPC" "Horizon Falloff" (`.Float` (`/ThoughtfishCoalaPlugin/Blueprints/Library/BP_BF_Coala.GetFloatByCoalaScaling` self (`self.FogHorizon Falloff`)))))

(fn `SetFogColor`
  (params (Hour :type Integer) (Minutes :type Integer))
  (bind _fog_color (`self.Fog Color`))
  (`/Engine/EditorBlueprintResources/StandardMacros.IsValid` _fog_color
    (:`Is Valid`
      (`KismetMaterialLibrary.SetVectorParameterValue` "/ThoughtfishCoalaPlugin/Materials/MPC.MPC" "Fog Color" (`CurveLinearColor.GetLinearColorValue` _fog_color (+ (`KismetMathLibrary.Conv_IntToDouble` Hour) (`KismetMathLibrary.MapRangeUnclamped` (`KismetMathLibrary.Conv_IntToDouble` Minutes) 0.0 59.0 0.0 1.0)))))))

(fn `SetMoonOpacity`
  (params (Hours :type Integer) (Minutes :type Integer))
  (bind _returnvalue (`KismetMathLibrary.Conv_IntToDouble` Minutes))
  (`/Engine/EditorBlueprintResources/StandardMacros.IsValid` (`self.SkySphere`)
    (:`Is Valid`
      (bind _arise (`self.IsMoonShowing` Hours Minutes))
      (if _arise
        (bind _arise_2 (`self.IsMoonArise ` Hours))
        (if _arise_2
          ;[1 1 1] Is Morning
          (if (<= Hours 12)
            ;[1 1 1] Morning
            (`/ThoughtfishCoalaPlugin/Blueprints/BP_Sky_Sphere_Coala.SetMoonOpacity` (`self.SkySphere`) (`KismetMathLibrary.MapRangeUnclamped` _returnvalue 0.0 (`KismetMathLibrary.Conv_IntToDouble` (`self.MoonMinutesTo`)) 1.0))
            (else
              ;[1 1 1] Evening
              (`/ThoughtfishCoalaPlugin/Blueprints/BP_Sky_Sphere_Coala.SetMoonOpacity` (`self.SkySphere`) (`KismetMathLibrary.MapRangeUnclamped` _returnvalue (`KismetMathLibrary.Conv_IntToDouble` (`self.MoonMinutesFrom`)) 59.0 0.0 1.0))))
          (else
            (`/ThoughtfishCoalaPlugin/Blueprints/BP_Sky_Sphere_Coala.SetMoonOpacity` (`self.SkySphere`) 1.0)))
        (else
          (`/ThoughtfishCoalaPlugin/Blueprints/BP_Sky_Sphere_Coala.SetMoonOpacity` (`self.SkySphere`) 0.0))))))

(fn `SetMoonPhaseFn`
  (params (MoonPhase :type "/ThoughtfishCoalaPlugin/Blueprints/types/MoonPhase Enum" :default "NewEnumerator5"))
  (`/Engine/EditorBlueprintResources/StandardMacros.IsValid` (`self.SkySphere`)
    (:`Is Valid`
      (`/ThoughtfishCoalaPlugin/Blueprints/BP_Sky_Sphere_Coala.SetMoonPhase` (`self.SkySphere`) MoonPhase))))

(fn `SetSunMoonIntensity`
  (params (DirectionalLight :type "DirectionalLight Object Reference") (IntensityCurve :type "CurveFloat Object Reference") (ColorCurve :type "CurveLinearColor Object Reference") (Hours :type Integer) (Minutes :type Integer))
  (locals (TempSunIntensity :type "Float (double-precision)" :default 0.0))
  (bind _tempsunintensity (`local.TempSunIntensity`))
  (if (and (`KismetSystemLibrary.IsValid` DirectionalLight) (`KismetSystemLibrary.IsValid` IntensityCurve) (`KismetSystemLibrary.IsValid` ColorCurve))
    (set `local.TempSunIntensity` (+ (`KismetMathLibrary.Conv_IntToDouble` Hours) (`KismetMathLibrary.MapRangeUnclamped` (`KismetMathLibrary.Conv_IntToDouble` Minutes) 0.0 59.0 0.0 1.0)))
    (`LightComponent.SetIntensity` (`Light.LightComponent` DirectionalLight) (`CurveFloat.GetFloatValue` IntensityCurve _tempsunintensity))
    (`LightComponent.SetLightColor` (`Light.LightComponent` DirectionalLight) (`CurveLinearColor.GetLinearColorValue` ColorCurve _tempsunintensity) true)))

(fn `SetupLight`
  (`/Engine/EditorBlueprintResources/StandardMacros.IsValid` (`self.SunDirectionalLight`)
    (:`Is Valid`
      (`/Engine/EditorBlueprintResources/StandardMacros.IsValid` (`self.SkySphere`)
        (:`Is Valid`
          (set `/Engine/EngineSky/BP_Sky_Sphere.Directional light actor` (`self.SunDirectionalLight`) (`self.SkySphere`)))))))

(fn `SetupSkySphere`
  (bind _skysphere (`self.SkySphere`))
  (`/Engine/EditorBlueprintResources/StandardMacros.IsValid` (`self.SkySphere`)
    (:`Is Valid`
      ;[1 1 1] Set Color Curves
      (`/Engine/EditorBlueprintResources/StandardMacros.IsValid` (`self.CoalaHorizontColor`)
        (:`Is Valid`
          (set `/Engine/EngineSky/BP_Sky_Sphere.Horizon color curve` (`self.CoalaHorizontColor`) (`self.SkySphere`)))
        (:`Is Not Valid`
          _))
      (`/Engine/EditorBlueprintResources/StandardMacros.IsValid` (`self.CoalaZenithColor`)
        (:`Is Valid`
          (set `/Engine/EngineSky/BP_Sky_Sphere.Zenith color curve` (`self.CoalaZenithColor`) (`self.SkySphere`)))
        (:`Is Not Valid`
          _))
      (`/Engine/EditorBlueprintResources/StandardMacros.IsValid` (`self.CoalaCloudColor`)
        (:`Is Valid`
          (set `/Engine/EngineSky/BP_Sky_Sphere.Cloud color curve` (`self.CoalaCloudColor`) (`self.SkySphere`)))
        (:`Is Not Valid`
          _))
      ;[1 1 1] Set Sun
      (set `/Engine/EngineSky/BP_Sky_Sphere.Sun brightness` (`self.CoalaSunBrightness`) (`self.SkySphere`))
      (set `/ThoughtfishCoalaPlugin/Blueprints/BP_Sky_Sphere_Coala.UseSunMesh` (`self.UseSunMesh`) (`self.SkySphere`))
      (set `/ThoughtfishCoalaPlugin/Blueprints/BP_Sky_Sphere_Coala.DistanceOfSun` (`self.CoalaSunDistance`) (`self.SkySphere`))
      (set `/ThoughtfishCoalaPlugin/Blueprints/BP_Sky_Sphere_Coala.SunScale` (`self.CoalaSunScale`) (`self.SkySphere`))
      ;[1 1 1] Moon
      (set `/ThoughtfishCoalaPlugin/Blueprints/BP_Sky_Sphere_Coala.UseMoonMesh` (`self.UseMoonMesh`) (`self.SkySphere`))
      (set `/ThoughtfishCoalaPlugin/Blueprints/BP_Sky_Sphere_Coala.MoonScale` (`self.CoalaMoonScale`) (`self.SkySphere`))
      (set `/ThoughtfishCoalaPlugin/Blueprints/BP_Sky_Sphere_Coala.DistanceOfMoon` (`self.CoalaMoonDistance`) (`self.SkySphere`))
      (set `/ThoughtfishCoalaPlugin/Blueprints/BP_Sky_Sphere_Coala.MoonStartPostion` (`self.CoalaMoonStartPosition`) (`self.SkySphere`))
      ;[1 1 1] Clouds
      (set `/Engine/EngineSky/BP_Sky_Sphere.Cloud speed` (`self.CoalaCloudSpeed`) (`self.SkySphere`))
      (set `/Engine/EngineSky/BP_Sky_Sphere.Cloud opacity` (`self.CoalaCloudOpacity`) (`self.SkySphere`))
      ;[1 1 1] Stars
      (set `/Engine/EngineSky/BP_Sky_Sphere.Stars brightness` (`self.StarBightness`) (`self.SkySphere`))
      ;[1 1 1] Horizont
      (set `/ThoughtfishCoalaPlugin/Blueprints/BP_Sky_Sphere_Coala.HorizonFalloffFrom` (`self.HorizonFalloffFrom`) (`self.SkySphere`))
      (set `/ThoughtfishCoalaPlugin/Blueprints/BP_Sky_Sphere_Coala.HorizonFalloffTo` (`self.HorizonFalloffTo`) (`self.SkySphere`))
      (`/ThoughtfishCoalaPlugin/Blueprints/BP_Sky_Sphere_Coala.UpdateSettings` _skysphere)
      (`/ThoughtfishCoalaPlugin/Blueprints/BP_Sky_Sphere_Coala.CoalaScaling` _skysphere))))

(fn `SpawnWeatherParticalSystem`
  (params (WeatherSettings :type "/ThoughtfishCoalaPlugin/Blueprints/Structure/BP_ST_Weather_PE Structure"))
  (bind (_particlesystem _scalewithcoalascaling _overrideparticlecolor _particlecolor _paremetercolorname) (break `/ThoughtfishCoalaPlugin/Blueprints/Structure/BP_ST_Weather_PE` WeatherSettings))
  (bind (_player _exist) (`/ThoughtfishCoalaPlugin/Blueprints/Library/BP_BF_Coala.GetCoalaPlayer` self))
  (if _exist
    (`/Engine/EditorBlueprintResources/StandardMacros.IsValid` _particlesystem
      (:`Is Valid`
        (bind _returnvalue (`GameplayStatics.SpawnEmitterAttached` _particlesystem (`Character.CapsuleComponent` _player) "None" (0.0 0.0 0.0) (struct) (1.0 1.0 1.0) "SnapToTarget"))
        (bind _output_get (set `self.CurrentWeather` _returnvalue))
        (if _overrideparticlecolor
          (`ParticleSystemComponent.SetColorParameter` (`self.CurrentWeather`) _paremetercolorname _particlecolor))
        (if _scalewithcoalascaling
          (`SceneComponent.SetWorldScale3D` _output_get (`.Vector` (`/ThoughtfishCoalaPlugin/Blueprints/Library/BP_BF_Coala.GetVectorByCoalaScaling` self (1.0 1.0 1.0)))))))))

(fn `UserConstructionScript`
  (`self.SetupLight`)
  (`self.UpdateManually`)
  (if (`self.UseDevmode`)
    (`self.SetMoonPhase` (`self.DevMoonPhase`))))
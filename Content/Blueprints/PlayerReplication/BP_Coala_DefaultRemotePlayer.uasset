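; Default actor representing a remote player, moving it toward replicated world positions with matching move and idle animations.
; MoveToPosition computes a velocity once per new target, scaled by distance above a minimum speed and capped at the distance.
; Animation play rate follows that speed.
; Tick advances the actor, snaps it to terrain, faces the target and switches to idle within one unit.
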(event `self.ReceiveTick`
  (params (DeltaSeconds :type "Float (single-precision)"))
  (`self.Update Movement` DeltaSeconds))

(fn `ComputeMoveDisp`
  (params (targetLocation :type "Vector Structure"))
  (returns (moveDispPerSecond :type "Vector Structure"))
  (bind _minmovementspeedinunits (`self.minMovementSpeedInUnits`))
  (bind _returnvalue (- targetLocation (`self.K2_GetActorLocation`)))
  (bind _returnvalue_2 (`KismetMathLibrary.VSize` _returnvalue))
  (return (* (/ _returnvalue _returnvalue_2) (`KismetMathLibrary.FMin` _returnvalue_2 (+ _minmovementspeedinunits (* (- _returnvalue_2 _minmovementspeedinunits) (`self.percentageOfTargetDistanceAsSpeed`)))))))

(fn `MoveToPosition`
  (params (NewWorldPosition :type "Vector Structure"))
  (bind _skeletalmesh (`self.SkeletalMesh`))
  (if (and (!= (`self.targetLocation`) NewWorldPosition) (> (`KismetMathLibrary.Vector_Distance` NewWorldPosition (`self.K2_GetActorLocation`)) 1.0))
    (bind _output_get (set `self.targetLocation` NewWorldPosition))
    (bind _movedisppersecond (`self.ComputeMoveDisp` _output_get))
    (set `self.moveDispPerSecond` _movedisppersecond)
    (set `self.isMoving` true)
    (`SkeletalMeshComponent.PlayAnimation` _skeletalmesh (`self.MoveAnimation`) true)
    (`SkeletalMeshComponent.SetPlayRate` _skeletalmesh (/ (`KismetMathLibrary.VSize` (`self.moveDispPerSecond`)) (`self.unrealUnitsPerSecondMovedInAnim`)))))

(fn `Update Movement`
  (params (DeltaSeconds :type "Float (double-precision)"))
  (locals (oldPosition :type "Vector Structure"))
  (if (`self.isMoving`)
    (bind _output_get (set `local.oldPosition` (`self.K2_GetActorLocation`)))
    (`self.K2_SetActorLocation` (`CoalaBlueprintUtility.GetTerrainPositionWithoutArea` (+ _output_get (* (`self.moveDispPerSecond`) DeltaSeconds)) self))
    (if (< (`KismetMathLibrary.Vector_DistanceSquared` (`self.K2_GetActorLocation`) (`self.targetLocation`)) 1.0)
      (set `self.isMoving` false)
      (`SkeletalMeshComponent.PlayAnimation` (`self.SkeletalMesh`) (`self.IdleAnimation`) true)
      (else
        (`self.K2_SetActorRotation` (`KismetMathLibrary.FindLookAtRotation` (`local.oldPosition`) (`self.targetLocation`)))))))

(fn `UserConstructionScript`)